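; CheckPoint1_BP is a level goal that completes the current map when an actor overlaps it.
; It flags player pawn 0 as IsGoal without checking which actor overlapped, shows the GravityRoomGoal_WG widget and plays a clap sound.
; When the WaitOpenLevel timeline finishes, it matches the current level name against map enum entry names to open the next one, or ResultMap after the last.
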(event `self.ReceiveActorBeginOverlap`
  (params (OtherActor :type "Actor Object Reference"))
  (bind _returnvalue (enumcount `/Game/Blueprint/MapEnum`))
  (bind _asplayer_bp (cast `/Game/Blueprint/player_BP` (`GameplayStatics.GetPlayerPawn` 0)))
  (set `/Game/Blueprint/player_BP.IsGoal` true _asplayer_bp)
  (`|ExecutionSequence`
    (:`then_0`
      (bind _returnvalue_2 (`|CreateWidget` "/Game/Blueprint/GravityRoomGoal_WG.GravityRoomGoal_WG_C"))
      (`UserWidget.AddToViewport` _returnvalue_2 0)
      (`GameplayStatics.PlaySound2D` "/Game/Sounds/clap.clap" 1.0 1.0 0.0 null null)
      (`Timeline|WaitOpenLevel`
        (:`Finished`
          (bind _returnvalue_3 (`GameplayStatics.GetCurrentLevelName` true))
          (for _index (range (+ _returnvalue 1))
            (bind _returnvalue_4 (cast `/Game/Blueprint/MapEnum` (`KismetMathLibrary.Conv_IntToByte` _index)))
            (bind _output_get (set `self.MapNum` _returnvalue_4))
            (if (`KismetStringLibrary.EqualEqual_StrStr` (`|GetEnumeratorNameAsString` _output_get) _returnvalue_3)
              (bind _returnvalue_5 (+ _returnvalue_4 1))
              (if (== _returnvalue_5 (`KismetMathLibrary.Conv_IntToByte` _returnvalue))
                (`GameplayStatics.OpenLevel` "ResultMap")
                (else
                  (bind _output_get_2 (set `self.MapNum` (cast `/Game/Blueprint/MapEnum` _returnvalue_5)))
                  (`GameplayStatics.OpenLevel` (`KismetStringLibrary.Conv_StringToName` (`|GetEnumeratorNameAsString` _output_get_2))))))))))))

(fn `UserConstructionScript`)