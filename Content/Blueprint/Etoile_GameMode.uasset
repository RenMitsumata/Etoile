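; Game mode for the Etoile level that plays an intro camera cinematic when play begins.
; It views through the first CheckPoint1_BP actor while a timeline animates its camera FOV, then blends to the player pawn over an eased transition and sets IsEndCine.
; A second timeline runs in parallel, stopping player movement and disabling input every update, then re-enables input when it finishes.
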(event `self.ReceiveBeginPlay`
  (bind _returnvalue (`GameplayStatics.GetPlayerController` 0))
  (bind _asplayer_bp (cast `/Game/Blueprint/player_BP` (`GameplayStatics.GetPlayerPawn` 0) :!pure true))
  (`|ExecutionSequence`
    (:`then_0`
      (bind _outactors (`GameplayStatics.GetAllActorsOfClass` "/Game/Blueprint/CheckPoint1_BP.CheckPoint1_BP_C"))
      (bind _output (`|GetArrayItem` _outactors))
      (`PlayerController.SetViewTargetWithBlend` _returnvalue _output 0.0 "VTBlend_Linear" 0.0 false)
      (bind (_direction `_新規track_0`) (`Timeline|FOVTimeline`)
        (:`Update`
          (`CameraComponent.SetFieldOfView` (`/Game/Blueprint/CheckPoint1_BP.Camera` _output) `_新規track_0`))
        (:`Finished`
          (`PlayerController.SetViewTargetWithBlend` _returnvalue _asplayer_bp 5.0 "VTBlend_EaseOut" 0.5 false)
          (set `self.IsEndCine` true))))
    (:`then_1`
      (`Timeline|タイムライン_0`
        (:`Update`
          (`NavMovementComponent.StopActiveMovement` (`Character.CharacterMovement` _asplayer_bp))
          (`self.DisableInput` _asplayer_bp _returnvalue))
        (:`Finished`
          (`self.EnableInput` _asplayer_bp null)
          (`KismetSystemLibrary.PrintString` "end" false false))))))

(fn `UserConstructionScript`)