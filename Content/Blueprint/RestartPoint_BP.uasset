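; RestartPoint_BP is a hazard point that fails the player and restarts the game when its Hit event fires.
; Each Hit flags the player's IsMiss, while a DoOnce gate plays a shock sound and adds a Fade_WG widget.
; A timeline drives the widget image's opacity, then calls RestartGame on Etoile_GameMode and resets the gate.
; An unconnected chain for moving the player back to StartLocation never runs.
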(event `self.ReceiveHit`
  (params (MyComp :type "PrimitiveComponent Object Reference") (Other :type "Actor Object Reference") (OtherComp :type "PrimitiveComponent Object Reference") (bSelfMoved :type Boolean) (HitLocation :type "Vector Structure") (HitNormal :type "Vector Structure") (NormalImpulse :type "Vector Structure") (Hit :type "HitResult Structure (by ref)"))
  (`|ExecutionSequence`
    (:`then_0`
      (`/Engine/EditorBlueprintResources/StandardMacros.DoOnce` false :!label _label
        (:`Completed`
          (`GameplayStatics.PlaySound2D` "/Game/Sounds/shock.shock" 1.0 1.0 0.0 null null)
          (bind _returnvalue (`|CreateWidget` "/Game/Blueprint/fade_WG.fade_WG_C"))
          (`UserWidget.AddToViewport` _returnvalue 0)
          (bind (_direction `_新規track_0`) (`Timeline|タイムライン_0`)
            (:`Update`
              (`Image.SetOpacity` (`/Game/Blueprint/fade_WG.Image_39` _returnvalue) `_新規track_0`))
            (:`Finished`
              (`GameMode.RestartGame` (cast `/Game/Blueprint/Etoile_GameMode` (cast `GameMode` (`GameplayStatics.GetGameMode`) :!pure true) :!pure true))
              (goto _label :!via `Reset`))))))
    (:`then_1`
      (set `/Game/Blueprint/player_BP.IsMiss` true (cast `/Game/Blueprint/player_BP` (`GameplayStatics.GetPlayerPawn` 0) :!pure true)))))

(fn `UserConstructionScript`)