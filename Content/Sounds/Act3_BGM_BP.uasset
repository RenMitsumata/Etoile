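; Background music controller for Act 3 that plays the stage track and stops it when the player misses.
; BeginPlay spawns the Act3 sound as 2D audio and stores the audio component.
; Tick loops the track by spawning a new sound whenever the stored one is not playing.
; Tick also polls IsMiss on player_BP and pauses the music when set, commented as landing on the floor.
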(event `self.ReceiveBeginPlay`
  ;[1 1 1] ステージ開始時にサウンドスタート
  (bind _returnvalue (`GameplayStatics.SpawnSound2D` "/Game/Sounds/act3.act3" 1.0 1.0 0.0 null false false))
  (set `self.Act3_BGM` _returnvalue))

(event `self.ReceiveTick`
  (params (DeltaSeconds :type "Float (single-precision)"))
  (`|ExecutionSequence`
    (:`then_0`
      ;[1 1 1] サウンドが止まったら再度始めから再生（ループ再生）
      (if (not (`AudioComponent.IsPlaying` (`self.Act3_BGM`)))
        (bind _returnvalue (`GameplayStatics.SpawnSound2D` "/Game/Sounds/act3.act3" 1.0 1.0 0.0 null false false))
        (set `self.Act3_BGM` _returnvalue)))
    (:`then_1`
      ;[1 1 1] 床に着地したら音楽停止
      (bind _asplayer_bp (cast `/Game/Blueprint/player_BP` (`GameplayStatics.GetPlayerPawn` 0)))
      (if (`/Game/Blueprint/player_BP.IsMiss` _asplayer_bp)
        (`AudioComponent.SetPaused` (`self.Act3_BGM`) true)))))

(fn `UserConstructionScript`)