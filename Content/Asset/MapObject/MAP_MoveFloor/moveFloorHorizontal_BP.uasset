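; Horizontally moving floor map object that shifts back and forth along the world Y axis around its placed position.
; On BeginPlay it stores its start location, then plays the 変動値 timeline, whose Sincurve track is scaled into a Y offset applied without sweep on each update.
; An older frame-counter movement that flips direction periodically remains in the graph but is never executed, and Tick is empty.
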(event `self.ReceiveBeginPlay`
  (set `self.startLocate` (`self.K2_GetActorLocation`))
  (bind (_direction _sincurve) (`Timeline|変動値`)
    (:`Update`
      (`self.K2_SetActorLocation` (+ (`self.startLocate`) (`KismetMathLibrary.MakeVector` 0.0 (* _sincurve 100.0)))))))

(event `self.ReceiveTick`
  (params (DeltaSeconds :type "Float (single-precision)")))

(fn `UserConstructionScript`)