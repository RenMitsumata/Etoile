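; RotateFloor_BP is a map-object floor meant to tilt according to player position and gravity, though its rotation logic is currently disconnected.
; BeginPlay only caches its GravityMovementComponent and zeroes the rotation; Hit is empty.
; The unused graph takes roll from a tilt-speed Timeline, flips it when player side on Y matches downward-gravity state, and applies world rotation.
; Helper functions supply both checks and expose an IsReverse flag.
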(event `self.ReceiveBeginPlay`
  ;[1 1 1] 初期化
  (set `self.NewVar_4` (`self.GetComponentByClass` "/Script/DirGravity.GravityMovementComponent"))
  (set `self.Rotation` (struct)))

(event `self.ReceiveHit`
  (params (MyComp :type "PrimitiveComponent Object Reference") (Other :type "Actor Object Reference") (OtherComp :type "PrimitiveComponent Object Reference") (bSelfMoved :type Boolean) (HitLocation :type "Vector Structure") (HitNormal :type "Vector Structure") (NormalImpulse :type "Vector Structure") (Hit :type "HitResult Structure (by ref)"))
  ;[1 1 1] ヒットイベント
)

(fn `get反転`
  (returns (isReverse :type Boolean))
  (return (`self.isReverse`)))

(fn `UserConstructionScript`)

(fn `プレイヤーの位置`
  (returns (is_Left :type Boolean))
  (return (> (.y (.location (`self.GetTransform`))) (.y (.location (`self.GetTransform` (`GameplayStatics.GetPlayerCharacter` 0)))))))

(fn `重力判定`
  (returns (is_GravityMinus :type Boolean))
  (bind (_returnvalue_x _returnvalue_y _returnvalue_z) (`KismetMathLibrary.BreakVector` (`GravityMovementComponent.GetGravityDirection` (`self.GetComponentByClass` (`GameplayStatics.GetPlayerCharacter` 0) "/Script/DirGravity.GravityMovementComponent") false)))
  (return (< _returnvalue_z 0.0)))